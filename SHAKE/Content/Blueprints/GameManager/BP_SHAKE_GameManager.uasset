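; SHAKE's game instance, which manages save data, startup display settings, online session flow and voice-chat muting.
; Init loads or creates the save and applies scalability and windowed fullscreen; Shutdown saves and leaves any session.
; Accepted invites pass a DoOnce guard, then destroy and join sessions, except for hosts already in one.
; Network errors trigger NetDisconnect: hosts disconnect clients before returning to MainMenu; clients notify the server.
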(event Custom|Save
  (bind _savefile (Variables|SaveData|GetSaveFile))
  ;[0.9911 0.03955 0.03955] SHUTDOWN
  (Variables|/Game/Blueprints/SaveData/BP_SHAKE_SaveFile.BP_SHAKE_SaveFile_C|SetSaveData _savefile (Variables|SaveData|GetSaveData))
  (SaveGame|SaveGametoSlot _savefile "SHAKE_SaveFile"))

(event Custom|NetDisconnect
  ;[0.7835 0.03071 0.03071] NET DISCONNECT
  (if (CallFunction|IsHost)
    (for _array_element (Variables|/Script/Engine.GameStateBase|GetPlayerArray (CallFunction|GetGameState))
      (if (!= (CallFunction|MyPlayerController) (.AsPlayer%20Controller (Utilities|Casting|CastToBP_SHAKE_PlayerController (Game|GetPlayerController _array_element))))
        (Default|ClientDisconnect (.AsPlayer%20Controller (Utilities|Casting|CastToBP_SHAKE_PlayerController (Game|GetPlayerController _array_element))))))
    (Utilities|FlowControl|Delay 1.0)
    (|DestroySession (CallFunction|MyPlayerController)
      (:OnSuccess
        _)
      (:OnFailure
        _))
    (Game|OpenLevel(byObjectReference) "/Game/Levels/MainMenu.MainMenu")
    (else
      (Default|ServerDisconnect (CallFunction|MyPlayerController)))))

(event EventInit
  ;[0.9911 0.03955 0.03955] INIT
  (|CallParentFunction)
  (bind _returnvalue (SaveGame|LoadGamefromSlot "SHAKE_SaveFile"))
  (Utilities|IsValid _returnvalue
    (:Is%20Valid
      (bind _output_get (Variables|SaveData|SetSaveFile (.AsSave%20File (Utilities|Casting|CastToBP_SHAKE_SaveFile _returnvalue))))
      (Variables|SaveData|SetSaveData (Variables|/Game/Blueprints/SaveData/BP_SHAKE_SaveFile.BP_SHAKE_SaveFile_C|GetSaveData _output_get))
      (CallFunction|SetScalability (.scalabilityquality (CallFunction|GetPlayerSettings))))
    (:Is%20Not%20Valid
      (bind _returnvalue_2 (Game|ConstructObjectfromClass self "/Game/Blueprints/SaveData/BP_SHAKE_SaveFile.BP_SHAKE_SaveFile_C"))
      (Variables|SaveData|SetSaveFile _returnvalue_2)
      (CallFunction|SetScalability "NewEnumerator3")))
  (bind _returnvalue_3 (Settings|GetGameUserSettings))
  (Class|GameUserSettings|SetFullscreenMode _returnvalue_3 "WindowedFullscreen")
  (Class|GameUserSettings|SetScreenResolution _returnvalue_3 (Class|GameUserSettings|GetDesktopResolution _returnvalue_3))
  (Class|GameUserSettings|SetResolutionScaleNormalized _returnvalue_3 1.0)
  (Class|GameUserSettings|ApplySettings _returnvalue_3 false))

(event EventShutdown
  ;[0.9911 0.03955 0.03955] SHUTDOWN
  (|CallParentFunction)
  (CallFunction|Save)
  (bind _sessionstate (Class|AdvancedSessionsLibrary|GetSessionState))
  (if (Utilities|Enum|NotEqual(Enum) _sessionstate "NoSession")
    (CallFunction|NetDisconnect)))

(event EventHandleNetworkError
  (params (FailureType :type ENetworkFailure%20Enum :default "NetDriverAlreadyExists") (bIsServer :type Boolean))
  ;[0.9911 0.03955 0.03955] NET / TRAVEL ERROR
  (CallFunction|NetDisconnect))

(event EventHandleTravelError
  (params (FailureType :type ETravelFailure%20Enum :default "NoLevel"))
  ;[0.9911 0.03955 0.03955] NET / TRAVEL ERROR
  (CallFunction|NetDisconnect))

(event EventOnSessionInviteAccepted
  (params (LocalPlayerNum :type Integer) (PersonInvited :type BP%20Unique%20Net%20Id%20Structure) (SessionToJoin :type Blueprint%20Session%20Result%20Structure%20%28by%20ref%29))
  (bind _playercontroller (CallFunction|MyPlayerController))
  ;[0.9911 0.03955 0.03955] INVITE
  (Utilities|FlowControl|DoOnce false :!label _label
    (:Completed
      (bind _sessionstate (Class|AdvancedSessionsLibrary|GetSessionState))
      (if (Utilities|Enum|Equal(Enum) _sessionstate "NoSession")
        _
        (elif (CallFunction|IsHost)
          (Audio|PlaySound2D "/Game/Sounds/New/SHAKE_Deny.SHAKE_Deny" (CallFunction|GetSoundVolume) 1.0 0.0 0 0)
          (goto _label Reset)
          (else
            _)))
      (|DestroySession _playercontroller
        (:OnSuccess
          _)
        (:OnFailure
          _))
      (|JoinSession _playercontroller SessionToJoin
        (:then
          (Default|ClientSwapWidget (CallFunction|MyPlayerController) "/Game/Blueprints/Menus/WBP_SHAKE_Loading.WBP_SHAKE_Loading_C"))
        (:OnSuccess
          (Audio|PlaySound2D "/Game/Sounds/New/SHAKE_Spawn.SHAKE_Spawn" (CallFunction|GetSoundVolume) 1.0 0.0 0 0)
          (goto _label Reset))
        (:OnFailure
          (|DestroySession _playercontroller
            (:OnSuccess
              (goto _label Reset))
            (:OnFailure
              (goto _label Reset))))))))

(fn ToggleMute
  (bind _player (CallFunction|MyPlayer))
  ;[0.2874 0 0] Toggles muting voice input
  (if (Utilities|Enum|NotEqual(Enum) (.voicechatvolume (CallFunction|GetPlayerSettings)) "NewEnumerator7")
    (bind _output_get (Variables|ProximityChat|SetbMuted (not (Variables|ProximityChat|GetbMuted))))
    (Class|VOIPStatics|SetMicThreshold (Math|Float|SelectFloat 1e+02 0.05 _output_get))
    (Utilities|IsValid _player
      (:Is%20Valid
        (Rendering|SetVisibility (Variables|/Game/Blueprints/Player/BP_SHAKE_Player.BP_SHAKE_Player_C|GetChatIcon _player) false false)))))