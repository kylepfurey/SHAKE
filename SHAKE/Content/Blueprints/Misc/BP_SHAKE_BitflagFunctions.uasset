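; Blueprint helper functions for testing, toggling, adding and removing bitflags in byte values, plus building a flag from a bit index.
; Each converts to integers for bitwise math and back to bytes, with the index helper raising two to that power.
; Toggle, add and remove write to the by-reference value and return it.
; RemoveFlag ORs with the inverted flag instead of ANDing, so it does not clear that bit.
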(fn HasFlag
  (params (Value :type Byte%20%28by%20ref%29) (Flag :type Byte :default 0))
  ;[0 0.1559 0.1274] Returns whether the given enumeration has the given flag
  (return (!= (Class|KismetMathLibrary|AndIntInt (Math|Conversions|ToInteger(Byte) Value) (Math|Conversions|ToInteger(Byte) Flag)) 0)))

(fn ToggleFlag
  (params (Value :type Byte%20%28by%20ref%29) (Flag :type Byte :default 1))
  ;[0 0.1559 0.1274] Flips the given bitflag
  (|SetBy-RefVar Value (Math|Conversions|ToByte(Integer) (Class|KismetMathLibrary|XorIntInt (Math|Conversions|ToInteger(Byte) Value) (Math|Conversions|ToInteger(Byte) Flag))))
  (return Value))

(fn AddFlag
  (params (Value :type Byte%20%28by%20ref%29) (Flag :type Byte :default 1))
  ;[0 0.1559 0.1274] Adds the given bitflag
  (|SetBy-RefVar Value (Math|Conversions|ToByte(Integer) (Class|KismetMathLibrary|OrIntInt (Math|Conversions|ToInteger(Byte) Value) (Math|Conversions|ToInteger(Byte) Flag))))
  (return Value))

(fn RemoveFlag
  (params (Value :type Byte%20%28by%20ref%29) (Flag :type Byte :default 1))
  ;[0 0.1559 0.1274] Removes the given bitflag
  (|SetBy-RefVar Value (Math|Conversions|ToByte(Integer) (Class|KismetMathLibrary|OrIntInt (Math|Conversions|ToInteger(Byte) Value) (Class|KismetMathLibrary|NotInt (Math|Conversions|ToInteger(Byte) Flag)))))
  (return Value))

(fn MakeLiteralBitflag
  (params (FlagIndex :type Byte :default 0))
  ;[0 0.1559 0.1274] Creates a bitflag literal from the given flag index
  (return (Math|Conversions|ToByte(Integer) (Math|Float|Truncate (Math|Float|Power 2.0 (Math|Conversions|ToFloat(Byte) FlagIndex))))))