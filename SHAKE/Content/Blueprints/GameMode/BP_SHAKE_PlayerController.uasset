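; Player controller for SHAKE that runs each player's match from pre-spawn countdown to end screen and return to the main menu.
; BeginPlay syncs Steam names and sets up input and widgets, with gates and DoOnce letting a forced start cut the announcer countdown.
; Server logic handles life-limited respawns and timeout results by kill count, while client events play feedback and record stats outside practice.
; It also handles scoreboard, emote, mute and quit input, plus weapon cooldowns.
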(event Custom|Server_RespawnPlayer
  (bind _gamemode (CallFunction|GetGameMode))
  (bind _self self)
  (bind _returnvalue (Class|GameModeBase|FindPlayerStart _gamemode _self))
  (bind _returnvalue_2 (Transformation|GetActorTransform _returnvalue))
  ;[0.956 0.0382 0.0382] RESPAWN PLAYER
  (Utilities|FlowControl|Delay (Math|Random|RandomFloatinRange 0.0 0.05))
  (if (and (not (Utilities|IsValid (Pawn|GetControlledPawn))) (> (Variables|Status|GetLives) 0))
    (bind _returnvalue_3 (Game|SpawnActorfromClass "/Game/Blueprints/Player/BP_SHAKE_Player.BP_SHAKE_Player_C" (Math|Transform|MakeTransform (.location _returnvalue_2) (.rotation _returnvalue_2) "1.000000,1.000000,1.000000") "AlwaysSpawn" "MultiplyWithRoot" self 0))
    (Pawn|Possess _returnvalue_3)))

(event Custom|Client_Disconnect
  ;[0.7835 0.03071 0.03071] DISCONNECT
  (|DestroySession self
    (:OnSuccess
      _)
    (:OnFailure
      _))
  (Game|OpenLevel(byObjectReference) "/Game/Levels/MainMenu.MainMenu"))

(event Custom|Client_CancelPlayerStart
  ;[0.7835 0.03071 0.03071] BEGIN PLAY
  (bind _foundwidgets (Widget|GetAllWidgetsOfClass "/Game/Blueprints/Player/HUD/WBP_SHAKE_PlayerSpawner.WBP_SHAKE_PlayerSpawner_C" true))
  (if (Utilities|Array|IsEmpty _foundwidgets)
    (Widget|RemovefromParent (Utilities|Array|Get(acopy) _foundwidgets))))

(event Custom|Client_SwapWidget
  (params (MenuClass :type WBP%20SHAKE%20Menu%20Base%20Class%20Reference))
  ;[1 0.03955 0.03955] SWAP WIDGET
  (bind _foundwidgets (Widget|GetAllWidgetsOfClass "/Game/Blueprints/Menus/Base/WBP_SHAKE_MenuBase.WBP_SHAKE_MenuBase_C" true))
  (for _array_element _foundwidgets
    (Default|SwapMenu _array_element MenuClass)))

(event Custom|Client_Lose
  (bind _playerstate (CallFunction|MyPlayerState))
  (bind _playerstate_2 (CallFunction|MyPlayerState))
  (bind _playercontroller (CallFunction|MyPlayerController))
  (bind _player (CallFunction|MyPlayer))
  (bind _hud (Variables|/Game/Blueprints/Player/BP_SHAKE_Player.BP_SHAKE_Player_C|GetHUD _player))
  ;[0.7835 0.03071 0.03071] WIN / LOSE
  (Utilities|FlowControl|Gate false :!label _label
    (:Exit
      (Audio|PlaySound2D "/Game/Sounds/New/SHAKE_Lose.SHAKE_Lose" (CallFunction|GetSoundVolume) 1.0 0.0 0 0)
      (Utilities|FlowControl|Sequence
        (:then_0
          (Utilities|SwitchonPractice
            (:NotPractice
              (Variables|/Game/Blueprints/GameMode/BP_SHAKE_PlayerState.BP_SHAKE_PlayerState_C|SetLoses _playerstate (+ (Variables|/Game/Blueprints/GameMode/BP_SHAKE_PlayerState.BP_SHAKE_PlayerState_C|GetLoses _playerstate) 1)))
            (:Practice
              _))
          (bind _returnvalue (UserInterface|CreateWidget "/Game/Blueprints/Player/HUD/WBP_SHAKE_PlayerEndScreen.WBP_SHAKE_PlayerEndScreen_C" _playercontroller false))
          (UserInterface|Viewport|AddtoViewport _returnvalue 2)
          (Utilities|FlowControl|Delay 1.0)
          (Audio|PlaySound2D (Utilities|Select :Index (Math|Random|RandomIntegerinRange 0 2) :Option%200 "/Game/Sounds/VoiceLines/Announcer/SHAKE_AnnouncerLose1.SHAKE_AnnouncerLose1" :Option%201 "/Game/Sounds/VoiceLines/Announcer/SHAKE_AnnouncerLose2.SHAKE_AnnouncerLose2" :Option%202 "/Game/Sounds/VoiceLines/Announcer/SHAKE_AnnouncerLose3.SHAKE_AnnouncerLose3") (CallFunction|GetVoiceVolume) 1.0 0.0 0 0)
          (Utilities|IsValid _player
            (:Is%20Valid
              (Utilities|IsValid _hud
                (:Is%20Valid
                  (Widget|RemovefromParent _hud))
                (:Is%20Not%20Valid
                  _)))
            (:Is%20Not%20Valid
              _))
          (Utilities|FlowControl|Sequence
            (:then_0
              (Utilities|FlowControl|Delay 7.0)
              (Networking|SwitchHasAuthority
                (:Authority
                  (Class|AdvancedSessionsLibrary|ServerTravel "MainMenu?listen" true false))))
            (:then_1
              (Utilities|SwitchonPractice
                (:NotPractice
                  (Utilities|FlowControl|Delay 1.0)
                  (Variables|/Game/Blueprints/GameMode/BP_SHAKE_PlayerState.BP_SHAKE_PlayerState_C|SetKills _playerstate_2 (+ (Variables|BP_SHAKE_PlayerController_C|GetCurrentKills (CallFunction|MyPlayerController)) (Variables|/Game/Blueprints/GameMode/BP_SHAKE_PlayerState.BP_SHAKE_PlayerState_C|GetKills _playerstate_2))))))))
        (:then_1
          (goto _label Close))
        (:then_2
          (Utilities|FlowControl|Gate false) ; enters at Close
        )))))

(event Custom|Client_Win
  (bind _playerstate (CallFunction|MyPlayerState))
  (bind _playerstate_2 (CallFunction|MyPlayerState))
  (bind _playercontroller (CallFunction|MyPlayerController))
  (bind _player (CallFunction|MyPlayer))
  (bind _hud (Variables|/Game/Blueprints/Player/BP_SHAKE_Player.BP_SHAKE_Player_C|GetHUD _player))
  ;[0.7835 0.03071 0.03071] WIN / LOSE
  (Utilities|FlowControl|Gate false :!label _label
    (:Exit
      (Audio|PlaySound2D (Utilities|Select :Index (Math|Random|RandomIntegerinRange 0 3) :Option%200 "/Game/Sounds/VoiceLines/Announcer/SHAKE_AnnouncerWin1.SHAKE_AnnouncerWin1" :Option%201 "/Game/Sounds/VoiceLines/Announcer/SHAKE_AnnouncerWin2.SHAKE_AnnouncerWin2" :Option%202 "/Game/Sounds/VoiceLines/Announcer/SHAKE_AnnouncerWin3.SHAKE_AnnouncerWin3") (CallFunction|GetVoiceVolume) 1.0 0.0 0 0)
      (Audio|PlaySound2D "/Game/Sounds/New/SHAKE_MarshMalo.SHAKE_MarshMalo" (CallFunction|GetMusicVolume) 1.0 0.0 0 0)
      (Utilities|FlowControl|Sequence
        (:then_0
          (Utilities|SwitchonPractice
            (:NotPractice
              (Variables|/Game/Blueprints/GameMode/BP_SHAKE_PlayerState.BP_SHAKE_PlayerState_C|SetWins _playerstate (+ 1 (Variables|/Game/Blueprints/GameMode/BP_SHAKE_PlayerState.BP_SHAKE_PlayerState_C|GetWins _playerstate))))
            (:Practice
              _))
          (bind _returnvalue (UserInterface|CreateWidget "/Game/Blueprints/Player/HUD/WBP_SHAKE_PlayerEndScreen.WBP_SHAKE_PlayerEndScreen_C" _playercontroller))
          (UserInterface|Viewport|AddtoViewport _returnvalue 2)
          (Utilities|FlowControl|Sequence
            (:then_0
              (Utilities|IsValid _player
                (:Is%20Valid
                  (Utilities|IsValid _hud
                    (:Is%20Valid
                      (Widget|RemovefromParent _hud))
                    (:Is%20Not%20Valid
                      _)))
                (:Is%20Not%20Valid
                  _))
              (Utilities|FlowControl|Sequence
                (:then_0
                  (Utilities|FlowControl|Delay 7.0)
                  (Networking|SwitchHasAuthority
                    (:Authority
                      (Class|AdvancedSessionsLibrary|ServerTravel "MainMenu?listen" true false))))
                (:then_1
                  (Utilities|SwitchonPractice
                    (:NotPractice
                      (Utilities|FlowControl|Delay 1.0)
                      (Variables|/Game/Blueprints/GameMode/BP_SHAKE_PlayerState.BP_SHAKE_PlayerState_C|SetKills _playerstate_2 (+ (Variables|BP_SHAKE_PlayerController_C|GetCurrentKills (CallFunction|MyPlayerController)) (Variables|/Game/Blueprints/GameMode/BP_SHAKE_PlayerState.BP_SHAKE_PlayerState_C|GetKills _playerstate_2))))))))
            (:then_1
              (Utilities|FlowControl|Delay 2.0)
              (Utilities|IsValid _player
                (:Is%20Valid
                  (Default|ServerPlayWinSound _player))))))
        (:then_1
          (goto _label Close))
        (:then_2
          (Utilities|FlowControl|Gate false) ; enters at Close
        )))))

(event Custom|Server_ForcePlayerStart
  (bind _gamestate (CallFunction|GetGameState))
  (bind _gamestate_2 (CallFunction|GetGameState))
  (bind _playerarray (Variables|/Script/Engine.GameStateBase|GetPlayerArray _gamestate_2))
  ;[0.7835 0.03071 0.03071] BEGIN PLAY
  (for _array_element _playerarray
    (CallFunction|ClientForcePlayerStart (.AsPlayer%20Controller (Utilities|Casting|CastToBP_SHAKE_PlayerController (Game|GetPlayerController _array_element))))
    (Variables|/Game/Blueprints/GameMode/BP_SHAKE_GameState.BP_SHAKE_GameState_C|SetRemainingPlayers _gamestate (Utilities|Array|Length _playerarray))
    (Variables|/Game/Blueprints/GameMode/BP_SHAKE_GameState.BP_SHAKE_GameState_C|SetbHasStarted _gamestate true)))

(event Custom|Client_PlayHitSound
  (params (bKill :type Boolean))
  (bind _player (CallFunction|MyPlayer))
  (bind (_volume _attenuation _concurrency) (CallFunction|GetSoundSettings))
  (bind _hud (Variables|/Game/Blueprints/Player/BP_SHAKE_Player.BP_SHAKE_Player_C|GetHUD _player))
  ;[0.9047 0.0356 0.0356] PLAY HIT SOUND
  (Audio|PlaySound2D (select bKill "/Game/Sounds/New/SHAKE_Kill.SHAKE_Kill" "/Game/Sounds/New/SHAKE_Hit.SHAKE_Hit") _volume 1.0 0.0 _concurrency 0)
  (Utilities|IsValid _player
    (:Is%20Valid
      (Utilities|IsValid _hud
        (:Is%20Valid
          (Default|HitMarker _hud))))))

(event Custom|Client_ForcePlayerStart
  (bind _voicevolume (CallFunction|GetVoiceVolume))
  ;[0.7835 0.03071 0.03071] BEGIN PLAY
  (bind _foundwidgets (Widget|GetAllWidgetsOfClass "/Game/Blueprints/Player/HUD/WBP_SHAKE_PlayerSpawner.WBP_SHAKE_PlayerSpawner_C" true))
  (if (not (Utilities|Array|IsEmpty _foundwidgets))
    (Default|ForcePlayerSpawn (Utilities|Array|Get(acopy) _foundwidgets))
    (Utilities|FlowControl|DoOnce false
      (:Completed
        (Input|AddMappingContext (PlayerController|LocalPlayerSubsystems|GetEnhancedInputLocalPlayerSubsystem (CallFunction|MyPlayerController)) "/Game/Blueprints/Player/Controls/IMC_SHAKE_PlayerControls.IMC_SHAKE_PlayerControls" 0 "(bIgnoreAllPressedKeysUntilRelease=True,bForceImmediately=False,bNotifyUserSettings=False)")
        (Utilities|FlowControl|Sequence
          (:then_0
            (CallFunction|ServerForcePlayerStart))
          (:then_1
            (Utilities|FlowControl|Sequence
              (:then_0
                (Utilities|FlowControl|Gate false) ; enters at Close
              )
              (:then_1
                (Utilities|FlowControl|Gate false) ; enters at Close
              )
              (:then_2
                (Utilities|FlowControl|Gate false) ; enters at Close
              )
              (:then_3
                (Utilities|IsValid (stale EventBeginPlay _returnvalue_6)
                  (:Is%20Valid
                    (Audio|Components|Audio|Stop (stale EventBeginPlay _returnvalue_6))
                    (Components|DestroyComponent (stale EventBeginPlay _returnvalue_6)))
                  (:Is%20Not%20Valid
                    _))
                (Utilities|IsValid (stale EventBeginPlay _returnvalue_7)
                  (:Is%20Valid
                    (Audio|Components|Audio|Stop (stale EventBeginPlay _returnvalue_7))
                    (Components|DestroyComponent (stale EventBeginPlay _returnvalue_7)))
                  (:Is%20Not%20Valid
                    _))
                (Utilities|IsValid (stale EventBeginPlay _returnvalue_8)
                  (:Is%20Valid
                    (Audio|Components|Audio|Stop (stale EventBeginPlay _returnvalue_8))
                    (Components|DestroyComponent (stale EventBeginPlay _returnvalue_8)))
                  (:Is%20Not%20Valid
                    _))
                (Utilities|IsValid (stale EventBeginPlay _returnvalue_9)
                  (:Is%20Valid
                    (Audio|Components|Audio|Stop (stale EventBeginPlay _returnvalue_9))
                    (Components|DestroyComponent (stale EventBeginPlay _returnvalue_9)))))))
          (:then_2
            (bind _returnvalue (UserInterface|CreateWidget "/Game/Blueprints/Player/HUD/WBP_SHAKE_Scoreboard.WBP_SHAKE_Scoreboard_C" self))
            (bind _output_get (Variables|Status|SetScoreboard _returnvalue))
            (UserInterface|Viewport|AddtoViewport _output_get 3)
            (Input|AddMappingContext (PlayerController|LocalPlayerSubsystems|GetEnhancedInputLocalPlayerSubsystem (CallFunction|MyPlayerController)) "/Game/Blueprints/Player/Controls/IMC_SHAKE_PersistentControls.IMC_SHAKE_PersistentControls" 0 "(bIgnoreAllPressedKeysUntilRelease=True,bForceImmediately=False,bNotifyUserSettings=False)")))))))

(event Custom|Server_Disconnect
  ;[0.7835 0.03071 0.03071] DISCONNECT
  (CallFunction|ClientDisconnect self))

(event Custom|TimeOut
  ;[1 0.03955 0.03955] TIME OUT
  (Networking|SwitchHasAuthority
    (:Authority
      (Utilities|FlowControl|DoOnce false
        (:Completed
          (if (and (> (Variables|Status|GetCurrentKills) 0) (> (Variables|Status|GetLives) 0))
            (bind _array_element (Utilities|Array|ForEachLoopwithBreak (Variables|/Script/Engine.GameStateBase|GetPlayerArray (CallFunction|GetGameState)) :!label _label)
              (:LoopBody
                (if (> (Variables|BP_SHAKE_PlayerController_C|GetCurrentKills (.AsPlayer%20Controller (Utilities|Casting|CastToBP_SHAKE_PlayerController (Game|GetPlayerController _array_element)))) (Variables|Status|GetCurrentKills))
                  (CallFunction|ClientLose)
                  (Utilities|FlowControl|Sequence
                    (:then_0
                      (goto _label_2 Close))
                    (:then_1
                      (goto _label Break)))))
              (:Completed
                (Utilities|FlowControl|Gate false :!label _label_2
                  (:Exit
                    (CallFunction|ClientWin)
                    (goto _label_2 Close)))))
            (else
              (CallFunction|ClientLose))))))))

(event Input|EnhancedActionEvents|EnhancedInputActionIA_SHAKE_Scoreboard
  (params (ActionValue :type Boolean) (ElapsedSeconds :type Float%20%28double-precision%29) (TriggeredSeconds :type Float%20%28double-precision%29) (InputAction :type Input%20Action%20Object%20Reference :default "/Game/Blueprints/Player/Controls/IA_SHAKE_Scoreboard.IA_SHAKE_Scoreboard"))
  (bind _scoreboard (Variables|Status|GetScoreboard))
  (bind _scoreboard_2 (Variables|/Game/Blueprints/Player/HUD/WBP_SHAKE_Scoreboard.WBP_SHAKE_Scoreboard_C|GetScoreboard _scoreboard))
  ;[0.956 0.0382 0.0382] SCOREBOARD
  (:Started
    (Utilities|IsValid _scoreboard_2
      (:Is%20Valid
        (Widget|SetVisibility _scoreboard_2 "SelfHitTestInvisible")
        (Default|Refresh _scoreboard))))
  (:Canceled
    (Utilities|IsValid _scoreboard :!label _label
      (:Is%20Valid
        (Widget|SetVisibility _scoreboard_2 "Hidden"))))
  (:Completed
    (goto _label)))

(event Input|EnhancedActionEvents|EnhancedInputActionIA_SHAKE_Mute
  (params (ActionValue :type Boolean) (ElapsedSeconds :type Float%20%28double-precision%29) (TriggeredSeconds :type Float%20%28double-precision%29) (InputAction :type Input%20Action%20Object%20Reference :default "/Game/Blueprints/Player/Controls/IA_SHAKE_Mute.IA_SHAKE_Mute"))
  (bind _gamemanager (CallFunction|GetGameManager))
  ;[0.956 0.0382 0.0382] MUTE
  (:Started
    (Default|ToggleMute _gamemanager :!label _label))
  (:Canceled
    (if (and (> ElapsedSeconds 0.25) (not (Variables|/Game/Blueprints/GameManager/BP_SHAKE_GameManager.BP_SHAKE_GameManager_C|GetbMuted _gamemanager))) :!label _label_2
      (goto _label)))
  (:Completed
    (goto _label_2)))

(event Input|EnhancedActionEvents|EnhancedInputActionIA_SHAKE_Emote1
  (params (ActionValue :type Boolean) (ElapsedSeconds :type Float%20%28double-precision%29) (TriggeredSeconds :type Float%20%28double-precision%29) (InputAction :type Input%20Action%20Object%20Reference :default "/Game/Blueprints/Player/Controls/IA_SHAKE_Emote1.IA_SHAKE_Emote1"))
  (bind _player (CallFunction|MyPlayer))
  ;[0.956 0.0382 0.0382] EMOTE
  (:Started
    (Utilities|IsValid _player
      (:Is%20Valid
        (Default|ServerSetEmote _player "NewEnumerator1")))))

(event Input|EnhancedActionEvents|EnhancedInputActionIA_SHAKE_Emote2
  (params (ActionValue :type Boolean) (ElapsedSeconds :type Float%20%28double-precision%29) (TriggeredSeconds :type Float%20%28double-precision%29) (InputAction :type Input%20Action%20Object%20Reference :default "/Game/Blueprints/Player/Controls/IA_SHAKE_Emote2.IA_SHAKE_Emote2"))
  (bind _player (CallFunction|MyPlayer))
  ;[0.956 0.0382 0.0382] EMOTE
  (:Started
    (Utilities|IsValid _player
      (:Is%20Valid
        (Default|ServerSetEmote _player "NewEnumerator2")))))

(event Input|EnhancedActionEvents|EnhancedInputActionIA_SHAKE_Emote4
  (params (ActionValue :type Boolean) (ElapsedSeconds :type Float%20%28double-precision%29) (TriggeredSeconds :type Float%20%28double-precision%29) (InputAction :type Input%20Action%20Object%20Reference :default "/Game/Blueprints/Player/Controls/IA_SHAKE_Emote4.IA_SHAKE_Emote4"))
  (bind _player (CallFunction|MyPlayer))
  ;[0.956 0.0382 0.0382] EMOTE
  (:Started
    (Utilities|IsValid _player
      (:Is%20Valid
        (Default|ServerSetEmote _player "NewEnumerator4")))))

(event Input|EnhancedActionEvents|EnhancedInputActionIA_SHAKE_Emote3
  (params (ActionValue :type Boolean) (ElapsedSeconds :type Float%20%28double-precision%29) (TriggeredSeconds :type Float%20%28double-precision%29) (InputAction :type Input%20Action%20Object%20Reference :default "/Game/Blueprints/Player/Controls/IA_SHAKE_Emote3.IA_SHAKE_Emote3"))
  (bind _player (CallFunction|MyPlayer))
  ;[0.956 0.0382 0.0382] EMOTE
  (:Started
    (Utilities|IsValid _player
      (:Is%20Valid
        (Default|ServerSetEmote _player "NewEnumerator3")))))

(event Input|EnhancedActionEvents|EnhancedInputActionIA_SHAKE_StopEmote
  (params (ActionValue :type Boolean) (ElapsedSeconds :type Float%20%28double-precision%29) (TriggeredSeconds :type Float%20%28double-precision%29) (InputAction :type Input%20Action%20Object%20Reference :default "/Game/Blueprints/Player/Controls/IA_SHAKE_StopEmote.IA_SHAKE_StopEmote"))
  (bind _player (CallFunction|MyPlayer))
  ;[0.956 0.0382 0.0382] EMOTE
  (:Started
    (Utilities|IsValid _player
      (:Is%20Valid
        (Default|ServerSetEmote _player "NewEnumerator0")))))

(event Input|EnhancedActionEvents|EnhancedInputActionIA_SHAKE_Quit
  (params (ActionValue :type Boolean) (ElapsedSeconds :type Float%20%28double-precision%29) (TriggeredSeconds :type Float%20%28double-precision%29) (InputAction :type Input%20Action%20Object%20Reference :default "/Game/Blueprints/Player/Controls/IA_SHAKE_Quit.IA_SHAKE_Quit"))
  ;[0.956 0.0382 0.0382] QUIT
  (:Started
    (bind _sessionstate (Class|AdvancedSessionsLibrary|GetSessionState))
    (if (Utilities|Enum|Equal(Enum) _sessionstate "NoSession")
      (Game|OpenLevel(byObjectReference) "/Game/Levels/MainMenu.MainMenu")
      (elif (not (CallFunction|IsHost))
        (Default|NetDisconnect (CallFunction|GetGameManager))))))

(event EventTick
  (params (DeltaSeconds :type Float%20%28single-precision%29))
  ;[0.7835 0.03071 0.03071] TICK
  (|CallParentFunction DeltaSeconds)
  (Variables|Status|SetGrenadeCooldown (- (Variables|Status|GetGrenadeCooldown) DeltaSeconds))
  (Variables|Status|SetRocketCooldown (- (Variables|Status|GetRocketCooldown) DeltaSeconds))
  (Variables|Status|SetShotgunCooldown (- (Variables|Status|GetShotgunCooldown) DeltaSeconds)))

(event EventDestroyed
  ;[1 0.03955 0.03955] DESTROYED
  (|CallParentFunction)
  (Default|Save (CallFunction|GetGameManager))
  (Networking|SwitchHasAuthority
    (:Authority
      (Default|PlayerDisconnected (CallFunction|GetGameMode) self))))

(event EventBeginPlay
  (bind _returnvalue (Ability|HasAuthority))
  (bind _playercontroller (CallFunction|MyPlayerController))
  (bind _playerstate (CallFunction|MyPlayerState))
  (bind _voicevolume (CallFunction|GetVoiceVolume))
  (bind _self self)
  (bind _uniquenetid (Class|AdvancedSessionsLibrary|GetUniqueNetID _self))
  (bind _returnvalue_2 (PlayerController|LocalPlayerSubsystems|GetEnhancedInputLocalPlayerSubsystem _playercontroller))
  ;[0.7835 0.03071 0.03071] BEGIN PLAY
  (|CallParentFunction)
  (Networking|SwitchHasAuthority
    (:Authority
      (Variables|Status|SetLives (Math|Conversions|ToInteger(Byte) (Utilities|String|EnumtoString (.StartingLives (Utilities|Struct|BreakF_SHAKE_GameRules (.HostSettings (Utilities|Struct|BreakF_SHAKE_SaveData (Variables|/Game/Blueprints/GameManager/BP_SHAKE_GameManager.BP_SHAKE_GameManager_C|GetSaveData (CallFunction|GetGameManager)))))))))
      (if (Pawn|IsLocalController) :!label _label
        (Utilities|FlowControl|Sequence
          (:then_0
            (Class|AdvancedSteamFriendsLibrary|RequestSteamFriendInfo _uniquenetid false :!label _label_2)
            (bind _returnvalue_3 (Class|AdvancedSteamFriendsLibrary|GetSteamPersonaName _uniquenetid))
            (Utilities|IsValid _playerstate
              (:Is%20Valid
                (Default|ServeronPlayerNameChanged _playerstate (Utilities|String|SelectString (Utilities|Platform|GetPlatformUserName) _returnvalue_3 (Utilities|Array|IsEmpty _returnvalue_3))))
              (:Is%20Not%20Valid
                _))
            (Utilities|FlowControl|Delay (Math|Random|RandomFloatinRange 0.1 1.0))
            (Utilities|IsValid self
              (:Is%20Valid
                (goto _label_2))))
          (:then_1
            (if (CallFunction|IsMainMenu)
              (Input|AddMappingContext _returnvalue_2 "/Game/Blueprints/Menus/Base/Controls/IMC_SHAKE_MenuControls.IMC_SHAKE_MenuControls" 0 "(bIgnoreAllPressedKeysUntilRelease=True,bForceImmediately=False,bNotifyUserSettings=False)")
              (else
                (bind _returnvalue_4 (UserInterface|CreateWidget "/Game/Blueprints/Player/HUD/WBP_SHAKE_PlayerSpawner.WBP_SHAKE_PlayerSpawner_C" self 3 true))
                (UserInterface|Viewport|AddtoViewport _returnvalue_4 1)
                (Utilities|FlowControl|Sequence
                  (:then_0
                    (Utilities|FlowControl|Delay (Math|Float|SelectFloat 8.0 7.5 _returnvalue))
                    (Utilities|FlowControl|DoOnce false
                      (:Completed
                        (Input|AddMappingContext _returnvalue_2 "/Game/Blueprints/Player/Controls/IMC_SHAKE_PlayerControls.IMC_SHAKE_PlayerControls" 0 "(bIgnoreAllPressedKeysUntilRelease=True,bForceImmediately=False,bNotifyUserSettings=False)")
                        (Utilities|FlowControl|Sequence
                          (:then_0
                            (CallFunction|ServerForcePlayerStart))
                          (:then_1
                            (Utilities|FlowControl|Sequence
                              (:then_0
                                (goto _label_3 Close))
                              (:then_1
                                (goto _label_4 Close))
                              (:then_2
                                (goto _label_5 Close))
                              (:then_3
                                (Utilities|IsValid (stale _returnvalue_6)
                                  (:Is%20Valid
                                    (Audio|Components|Audio|Stop (stale _returnvalue_6))
                                    (Components|DestroyComponent (stale _returnvalue_6)))
                                  (:Is%20Not%20Valid
                                    _))
                                (Utilities|IsValid (stale _returnvalue_7)
                                  (:Is%20Valid
                                    (Audio|Components|Audio|Stop (stale _returnvalue_7))
                                    (Components|DestroyComponent (stale _returnvalue_7)))
                                  (:Is%20Not%20Valid
                                    _))
                                (Utilities|IsValid (stale _returnvalue_8)
                                  (:Is%20Valid
                                    (Audio|Components|Audio|Stop (stale _returnvalue_8))
                                    (Components|DestroyComponent (stale _returnvalue_8)))
                                  (:Is%20Not%20Valid
                                    _))
                                (Utilities|IsValid (stale _returnvalue_9)
                                  (:Is%20Valid
                                    (Audio|Components|Audio|Stop (stale _returnvalue_9))
                                    (Components|DestroyComponent (stale _returnvalue_9)))))))
                          (:then_2
                            (bind _returnvalue_5 (UserInterface|CreateWidget "/Game/Blueprints/Player/HUD/WBP_SHAKE_Scoreboard.WBP_SHAKE_Scoreboard_C" self))
                            (bind _output_get (Variables|Status|SetScoreboard _returnvalue_5))
                            (UserInterface|Viewport|AddtoViewport _output_get 3)
                            (Input|AddMappingContext (PlayerController|LocalPlayerSubsystems|GetEnhancedInputLocalPlayerSubsystem (CallFunction|MyPlayerController)) "/Game/Blueprints/Player/Controls/IMC_SHAKE_PersistentControls.IMC_SHAKE_PersistentControls" 0 "(bIgnoreAllPressedKeysUntilRelease=True,bForceImmediately=False,bNotifyUserSettings=False)"))))))
                  (:then_1
                    (Utilities|FlowControl|Delay (Math|Float|SelectFloat 0.5 0.0 _returnvalue))
                    (bind _returnvalue_6 (Audio|SpawnSound2D "/Game/Sounds/VoiceLines/Announcer/SHAKE_AnnouncerStart_GetReady.SHAKE_AnnouncerStart_GetReady" _voicevolume 1.0 0.0 0))
                    (Utilities|FlowControl|Delay 3.5)
                    (Utilities|FlowControl|Gate false :!label _label_3
                      (:Exit
                        (bind _returnvalue_7 (Audio|SpawnSound2D "/Game/Sounds/VoiceLines/Announcer/SHAKE_AnnouncerStart_3.SHAKE_AnnouncerStart_3" _voicevolume 1.0 0.0 0))
                        (Utilities|FlowControl|Delay 1.5)
                        (Utilities|FlowControl|Gate false :!label _label_4
                          (:Exit
                            (bind _returnvalue_8 (Audio|SpawnSound2D "/Game/Sounds/VoiceLines/Announcer/SHAKE_AnnouncerStart_2.SHAKE_AnnouncerStart_2" _voicevolume 1.0 0.0 0))
                            (Utilities|FlowControl|Delay 1.0)
                            (Utilities|FlowControl|Gate false :!label _label_5
                              (:Exit
                                (bind _returnvalue_9 (Audio|SpawnSound2D "/Game/Sounds/VoiceLines/Announcer/SHAKE_AnnouncerStart_1.SHAKE_AnnouncerStart_1" _voicevolume 1.0 0.0 0)))))))))))))
          (:then_2
            (if (and (.bhud (CallFunction|GetPlayerSettings)) (not (CallFunction|IsMainMenu)))
              (bind _returnvalue_10 (UserInterface|CreateWidget "/Game/Blueprints/Player/HUD/WBP_SHAKE_KillFeed.WBP_SHAKE_KillFeed_C" self))
              (bind _output_get_2 (Variables|Status|SetKillFeed _returnvalue_10))
              (UserInterface|Viewport|AddtoViewport _output_get_2 3)))
          (:then_3
            (Input|AddMappingContext _returnvalue_2 "/Game/Blueprints/Player/Controls/IMG_SHAKE_Mute.IMG_SHAKE_Mute" 0 "(bIgnoreAllPressedKeysUntilRelease=True,bForceImmediately=False,bNotifyUserSettings=False)")))))
    (:Remote
      (if (and (Variables|/Game/Blueprints/GameMode/BP_SHAKE_GameState.BP_SHAKE_GameState_C|GetbHasStarted (CallFunction|GetGameState)) (not (CallFunction|IsMainMenu)))
        (if (Pawn|IsLocalController)
          (Default|NetDisconnect (CallFunction|GetGameManager)))
        (else
          (goto _label))))))

(fn ConstructionScript)

(fn SetCameraView
  (params (NewCamera :type Camera%20Actor%20Object%20Reference))
  (bind _returnvalue (Pawn|GetControlledPawn))
  (bind _asplayer (Utilities|Casting|CastToBP_SHAKE_Player _returnvalue))
  ;[0 0.3864 0.8796] Sets the player's camera view to the given camera actor
  (Utilities|IsValid NewCamera
    (:Is%20Valid
      (Game|Player|SetViewTargetwithBlend NewCamera 0.0 "VTBlend_Linear" 0.0 false)
      (bind _output_get (Variables|/Game/Blueprints/GameManager/BP_SHAKE_GameManager.BP_SHAKE_GameManager_C|SetCurrentCamera (CallFunction|GetGameManager) (Variables|/Script/Engine.CameraActor|GetCameraComponent NewCamera)))
      (return true _output_get))
    (:Is%20Not%20Valid
      (Utilities|IsValid _returnvalue
        (:Is%20Valid
          (Game|Player|SetViewTargetwithBlend _asplayer 0.0 "VTBlend_Linear" 0.0 false)
          (bind _output_get_2 (Variables|/Game/Blueprints/GameManager/BP_SHAKE_GameManager.BP_SHAKE_GameManager_C|SetCurrentCamera (CallFunction|GetGameManager) (Variables|/Game/Blueprints/Player/BP_SHAKE_Player.BP_SHAKE_Player_C|GetCamera _asplayer)))
          (return true _output_get_2))
        (:Is%20Not%20Valid
          (return false (Variables|/Game/Blueprints/GameManager/BP_SHAKE_GameManager.BP_SHAKE_GameManager_C|GetCurrentCamera (CallFunction|GetGameManager))))))))

(fn OnRepLives
  (bind _player (CallFunction|MyPlayer))
  (bind _hud (Variables|/Game/Blueprints/Player/BP_SHAKE_Player.BP_SHAKE_Player_C|GetHUD _player))
  ;[0.0137 0.7454 0.4179] Replicates the player's life count
  (Utilities|IsValid _player
    (:Is%20Valid
      (Utilities|IsValid _hud
        (:Is%20Valid
          (Default|UpdateLives _hud))))))

(fn OnRepCurrentKills
  (bind _player (CallFunction|MyPlayer))
  (bind _hud (Variables|/Game/Blueprints/Player/BP_SHAKE_Player.BP_SHAKE_Player_C|GetHUD _player))
  ;[0.0137 0.7454 0.4179] Replicates the player's kill count
  (Utilities|IsValid _player
    (:Is%20Valid
      (Utilities|IsValid _hud
        (:Is%20Valid
          (Default|UpdateKills _hud))))))