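; BP_SHAKE_Explosion is a short-lived explosion effect that flashes, grows and collapses before destroying itself.
; On BeginPlay it creates dynamic materials for two mesh slots, applies base, outer and inner emissive colors, and plays a sound at its location.
; Tick randomizes rotation every frame and scales uniformly by ExpandSpeed, which BeginPlay reverses and doubles after a brief delay so it shrinks faster than it grew.
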(event EventBeginPlay
  (bind (_volume _attenuation _concurrency) (CallFunction|GetSoundSettings))
  (bind _explosion (Variables|Default|GetExplosion))
  (bind _explosion_2 (Variables|Default|GetExplosion))
  (bind _returnvalue (Rendering|Material|GetMaterial _explosion 1))
  (bind _returnvalue_2 (Rendering|Material|GetMaterial _explosion_2 0))
  ;[1 0.03955 0.03955] BEGIN PLAY
  (|CallParentFunction)
  (bind _returnvalue_3 (Rendering|Material|CreateDynamicMaterialInstance _explosion_2 0 _returnvalue_2 (Utilities|String|StringToName (Utilities|GetDisplayName _returnvalue_2)) :!class /Script/Engine.PrimitiveComponent))
  (bind _returnvalue_4 (Rendering|Material|CreateDynamicMaterialInstance _explosion 1 _returnvalue (Utilities|String|StringToName (Utilities|GetDisplayName _returnvalue)) :!class /Script/Engine.PrimitiveComponent))
  (Rendering|Material|SetVectorParameterValue _returnvalue_3 "BaseColorParam" (Variables|Explosion|GetBaseColor) :!class /Script/Engine.MaterialInstanceDynamic)
  (Rendering|Material|SetVectorParameterValue _returnvalue_3 "EmissiveColorParam" (Variables|Explosion|GetEmissiveColor) :!class /Script/Engine.MaterialInstanceDynamic)
  (Rendering|Material|SetVectorParameterValue _returnvalue_4 "EmissiveColorParam" (Variables|Explosion|GetInnerEmissiveColor) :!class /Script/Engine.MaterialInstanceDynamic)
  (Audio|PlaySoundatLocation "/Game/Sounds/New/SHAKE_Explosion.SHAKE_Explosion" (Transformation|GetActorLocation) "0, 0, 0" _volume 1.0 0.0 "/Game/Sounds/Configuration/ExplosiveAttenuation.ExplosiveAttenuation" _concurrency 0 0)
  (Utilities|FlowControl|Delay 0.1)
  (Variables|Explosion|SetExpandSpeed (* -2.0 (Variables|Explosion|GetExpandSpeed)))
  (Utilities|FlowControl|Delay 0.1)
  (Actor|DestroyActor))

(event EventTick
  (params (DeltaSeconds :type Float%20%28single-precision%29))
  (bind _expandspeed (Variables|Explosion|GetExpandSpeed))
  ;[1 0.03955 0.03955] TICK
  (|CallParentFunction DeltaSeconds)
  (Transformation|SetActorRotation (Math|Random|RandomRotator true))
  (Transformation|SetActorScale3D (+ (Transformation|GetActorScale3D) (Math|Vector|MakeVector (* DeltaSeconds _expandspeed) (* DeltaSeconds _expandspeed) (* DeltaSeconds _expandspeed)))))

(fn ConstructionScript)