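; Player state for SHAKE that holds replicated Wins, Loses, Kills and Damage, and relays name changes and kill-feed entries by multicast.
; On BeginPlay it waits for a controller; a local one sends saved stats to the server and writes changes back to the GameManager's save data.
; Non-local controllers retry voice-talker registration each tick, then unmute.
; Damage replication refreshes the local HUD and tints name text from white toward red.
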(event Custom|Server_OnPlayerNameChanged
  (params (NewPlayerName :type String))
  ;[0.9647 0.0382 0.0382] PLAYER NAME
  (CallFunction|MulticastonPlayerNameChanged NewPlayerName))

(event Custom|Server_SetStats
  (params (Wins :type Integer) (Loses :type Integer) (Kills :type Integer))
  ;[0.9647 0.0382 0.0382] BEGIN PLAY
  (Variables|Stats|SetWins Wins)
  (Variables|Stats|SetLoses Loses)
  (Variables|Stats|SetKills Kills))

(event Custom|SaveStats
  (params (Wins :type Integer) (Loses :type Integer) (Kills :type Integer))
  ;[0.9647 0.0382 0.0382] BEGIN PLAY
  (bind _structout (Utilities|Struct|SetmembersinF_SHAKE_SaveData (Variables|/Game/Blueprints/GameManager/BP_SHAKE_GameManager.BP_SHAKE_GameManager_C|GetSaveData (CallFunction|GetGameManager)) Wins Loses Kills))
  (Variables|/Game/Blueprints/GameManager/BP_SHAKE_GameManager.BP_SHAKE_GameManager_C|SetSaveData (CallFunction|GetGameManager) _structout))

(event Custom|Multicast_OnPlayerNameChanged
  (params (NewPlayerName :type String))
  ;[0.9647 0.0382 0.0382] PLAYER NAME
  (Default|CallOnPlayerNameChanged NewPlayerName)
  (Variables|PlayerName|SetName (Utilities|String|StringToName NewPlayerName)))

(event Custom|Multicast_KillFeed
  (params (Killed :type BP%20SHAKE%20Player%20State%20Object%20Reference) (Killer :type BP%20SHAKE%20Player%20State%20Object%20Reference))
  (bind _playercontroller (CallFunction|MyPlayerController))
  (bind _killfeed (Variables|/Game/Blueprints/GameMode/BP_SHAKE_PlayerController.BP_SHAKE_PlayerController_C|GetKillFeed _playercontroller))
  ;[1 0.03955 0.03955] KILL FEED
  (Utilities|IsValid _killfeed
    (:Is%20Valid
      (Default|EnqueKillFeed _killfeed Killed Killer))))

(event EventBeginPlay
  (bind _returnvalue (Game|GetPlayerController))
  (bind _gamemanager (CallFunction|GetGameManager))
  (bind _self self)
  (bind _uniquenetid (Class|AdvancedSessionsLibrary|GetUniqueNetIDfromPlayerState _self))
  (bind _savedata (Variables|/Game/Blueprints/GameManager/BP_SHAKE_GameManager.BP_SHAKE_GameManager_C|GetSaveData _gamemanager))
  (bind (_playersettings _wins _loses _kills) (Utilities|Struct|BreakF_SHAKE_SaveData _savedata))
  ;[0.9647 0.0382 0.0382] BEGIN PLAY
  (|CallParentFunction)
  (Utilities|IsValid _returnvalue :!label _label
    (:Is%20Valid
      (if (Pawn|IsLocalController _returnvalue)
        (CallFunction|ServerSetStats _wins _loses _kills)
        (EventDispatchers|BindEventtoOnStatsChanged (delegate Custom|SaveStats))
        (else
          (bind _returnvalue_2 (Class|AdvancedVoiceLibrary|RegisterRemoteTalker _uniquenetid :!label _label_2))
          (if _returnvalue_2
            (Class|AdvancedVoiceLibrary|UnMuteRemoteTalker 0 _uniquenetid false)
            (else
              (Utilities|FlowControl|DelayUntilNextTick)
              (Utilities|IsValid self
                (:Is%20Valid
                  (goto _label_2))))))))
    (:Is%20Not%20Valid
      (Utilities|FlowControl|DelayUntilNextTick)
      (goto _label))))

(fn ConstructionScript)

(fn OnRepWins
  ;[0.01298 0.7305 0.4072] Replicates Wins
  (Default|CallOnStatsChanged (Variables|Stats|GetWins) (Variables|Stats|GetLoses) (Variables|Stats|GetKills)))

(fn OnRepLoses
  ;[0.0137 0.7379 0.4125] Replicates Loses
  (Default|CallOnStatsChanged (Variables|Stats|GetWins) (Variables|Stats|GetLoses) (Variables|Stats|GetKills)))

(fn OnRepDamage
  (bind _player (CallFunction|MyPlayer))
  (bind _returnvalue (PlayerState|GetPawn))
  (bind _returnvalue_2 (PlayerState|GetPawn))
  (bind _damage (Variables|Status|GetDamage))
  (bind _returnvalue_3 (/ _damage 1e+02))
  (bind _hud (Variables|/Game/Blueprints/Player/BP_SHAKE_Player.BP_SHAKE_Player_C|GetHUD _player))
  (bind _returnvalue_4 (Math|Float|Clamp(Float) _returnvalue_3))
  (bind _returnvalue_5 (- 1.0 _returnvalue_4))
  (bind _returnvalue_6 (* _returnvalue_5 255.0))
  (bind _returnvalue_7 (Math|Float|Round _returnvalue_6))
  (bind _returnvalue_8 (Math|Conversions|ToByte(Integer) _returnvalue_7))
  ;[0.03955 0.6654 0] Replicates the total number of remaining players
  (Utilities|IsValid _returnvalue
    (:Is%20Valid
      (if (Pawn|IsLocallyControlled _returnvalue)
        (Utilities|IsValid _player
          (:Is%20Valid
            (Utilities|IsValid _hud
              (:Is%20Valid
                (Default|UpdateDamage _hud))
              (:Is%20Not%20Valid
                _))))
        (else
          (Utilities|IsValid _returnvalue_2
            (:Is%20Valid
              _))))
      (Rendering|Components|TextRender|SetTextRenderColor (Variables|/Game/Blueprints/Player/BP_SHAKE_Player.BP_SHAKE_Player_C|GetPlayerNameText (.AsPlayer (Utilities|Casting|CastToBP_SHAKE_Player _returnvalue_2))) (Math|Color|MakeColor _returnvalue_8 _returnvalue_8 255 255)))))

(fn OnRepKills
  ;[0.01298 0.7305 0.4072] Replicates Kills
  (Default|CallOnStatsChanged (Variables|Stats|GetWins) (Variables|Stats|GetLoses) (Variables|Stats|GetKills)))