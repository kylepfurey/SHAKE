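; BP_SHAKE_BulletHole is a bullet hole mark that stays on the actor that was hit for a short, fixed lifetime.
; On BeginPlay it gives its Plane a random yaw, attaches itself to HitActor keeping world transform, and destroys itself after a delay.
; An opacity fade using a dynamic material and a per-tick loop is present but disconnected, so the mark disappears without fading.
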(event EventBeginPlay
  ;[1 0.03955 0.03955] BEGIN PLAY
  (|CallParentFunction)
  (Transformation|SetRelativeRotation (Variables|Default|GetPlane) (Math|Rotator|MakeRotator 0.0 0.0 (Math|Random|RandomFloatinRange 0.0 3.6e+02)) false false)
  (Utilities|FlowControl|Sequence
    (:then_0
      (Utilities|FlowControl|Delay 5.0)
      (Actor|DestroyActor))
    (:then_1
      (Transformation|AttachActorToActor (Variables|Hole|GetHitActor) "None" "KeepWorld" "KeepWorld" "KeepWorld" true))))

(fn ConstructionScript)