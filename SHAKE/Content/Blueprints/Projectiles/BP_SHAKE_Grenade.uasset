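; Bouncing grenade projectile that spins in flight and can gain launch speed from its owner's movement.
; The server explodes it on a fuse, on player contact (with direct damage to non-owners) or on impact once bounces run out.
; Explosions deal distance-scaled splash damage, credit the thrower and only push the owner.
; Multicasts spawn explosion, blast hole and bounce sound; pawn blocking starts shortly after leaving the owner.
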(event OnComponentHit(Collider)
  (params (HitComponent :type Primitive%20Component%20Object%20Reference) (OtherActor :type Actor%20Object%20Reference) (OtherComp :type Primitive%20Component%20Object%20Reference) (NormalImpulse :type Vector :default "0, 0, 0") (Hit :type Hit%20Result%20Structure%20%28by%20ref%29))
  ;[0.8228 0.03311 0.03311] COLLISION
  (Projectile|OnCollide OtherActor Hit))

(event OnComponentBeginOverlap(Collider)
  (params (OverlappedComponent :type Primitive%20Component%20Object%20Reference) (OtherActor :type Actor%20Object%20Reference) (OtherComp :type Primitive%20Component%20Object%20Reference) (OtherBodyIndex :type Integer) (bFromSweep :type Boolean) (SweepResult :type Hit%20Result%20Structure%20%28by%20ref%29))
  ;[0.8228 0.03311 0.03311] COLLISION
  (if (!= OtherActor (Components|GetOwner))
    (Projectile|OnCollide OtherActor SweepResult)))

(event OnComponentEndOverlap(Collider)
  (params (OverlappedComponent :type Primitive%20Component%20Object%20Reference) (OtherActor :type Actor%20Object%20Reference) (OtherComp :type Primitive%20Component%20Object%20Reference) (OtherBodyIndex :type Integer))
  ;[0.8228 0.03311 0.03311] COLLISION
  (Networking|SwitchHasAuthority
    (:Authority
      (if (== OtherActor (Components|GetOwner))
        (Utilities|FlowControl|Delay 0.1)
        (Collision|SetCollisionResponsetoChannel (Variables|Default|GetCollider) "ECC_Pawn" "ECR_Block")))))

(event Custom|Multicast_SpawnExplosion
  ;[1 0.03955 0.03955] SPAWN EXPLOSION
  (Game|SpawnActorfromClass "/Game/Blueprints/Projectiles/BP_SHAKE_Explosion.BP_SHAKE_Explosion_C" (Math|Transform|MakeTransform (Transformation|GetActorLocation) "0, 0, 0" "1.000000,1.000000,1.000000") "AlwaysSpawn" "MultiplyWithRoot" 0 (Variables|Explosion|GetBaseColor) (Variables|Explosion|GetEmissiveColor) (Variables|Explosion|GetInnerEmissiveColor) (* (/ (Variables|Projectile|GetExplosionRadius) 5e+02) 15.0) 0))

(event Custom|Multicast_SpawnBlastHole
  (params (WorldLocation :type Vector) (WorldNormal :type Vector) (HitActor :type Actor%20Object%20Reference))
  ;[1 0.03955 0.03955] SPAWN BLAST HOLE
  (Game|SpawnActorfromClass "/Game/Blueprints/Projectiles/BP_SHAKE_BlastHole.BP_SHAKE_BlastHole_C" (Math|Transform|MakeTransform WorldLocation (Math|Rotator|MakeRotfromZ WorldNormal) "1.000000,1.000000,1.000000") "AlwaysSpawn" "MultiplyWithRoot" 0 HitActor 0))

(event Custom|Multicast_PlayBumpSound
  (params (WorldPosition :type Vector))
  (bind (_volume _attenuation _concurrency) (CallFunction|GetSoundSettings))
  ;[1 0.03955 0.03955] PLAY BUMP SOUND
  (Audio|PlaySoundatLocation "/Game/Sounds/New/SHAKE_Bounce.SHAKE_Bounce" WorldPosition "0, 0, 0" _volume 1.0 0.0 _attenuation _concurrency 0 0))

(event EventBeginPlay
  (bind (_volume _attenuation _concurrency) (CallFunction|GetSoundSettings))
  (bind _returnvalue (Math|Random|RandomUnitVector))
  (bind _whoosh (Variables|Default|GetWhoosh))
  ;[0.8228 0.03311 0.03311] BEGIN PLAY
  (|CallParentFunction)
  (Audio|SpawnSoundAttached (Variables|Projectile|GetFireSound) (Variables|Default|GetCollider) "None" "0, 0, 0" "0, 0, 0" "KeepRelativeOffset" true _volume 1.0 0.0 _attenuation _concurrency)
  (Audio|Components|Audio|SetVolumeMultiplier _whoosh _volume :!class /Script/Engine.AudioComponent)
  (Audio|Components|Audio|Play _whoosh (Math|Random|RandomFloatinRange 1.0 5.0))
  (Variables|Projectile|SetDeltaRotation (Math|Rotator|MakeRotator (.x _returnvalue) (.y _returnvalue) (.z _returnvalue)))
  (Projectile|FollowPlayerVelocity)
  (Networking|SwitchHasAuthority
    (:Authority
      (Utilities|FlowControl|Delay (Variables|Projectile|GetExplosionDelay))
      (Utilities|IsValid self
        (:Is%20Valid
          (Projectile|Explode))))))

(event EventTick
  (params (DeltaSeconds :type Float%20%28single-precision%29))
  ;[0.8228 0.03311 0.03311] TICK
  (|CallParentFunction DeltaSeconds)
  (Transformation|AddRelativeRotation (Variables|Default|GetModel) (* (* (Variables|Projectile|GetDeltaRotation) 1e+03) DeltaSeconds) false false))

(fn ConstructionScript)

(fn Explode
  (bind _returnvalue (Transformation|GetActorLocation))
  (bind _explosionradius (Variables|Projectile|GetExplosionRadius))
  ;[0 0.3712 0.8469] Explodes this projectile, knocking and damaging all nearby players
  (Networking|SwitchHasAuthority
    (:Authority
      (Utilities|FlowControl|Sequence
        (:then_0
          (for _array_element (Variables|/Script/Engine.GameStateBase|GetPlayerArray (CallFunction|GetGameState))
            (Utilities|IsValid (PlayerState|GetPawn _array_element)
              (:Is%20Valid
                (if (< (Math|Vector|Distance(Vector) (+ (Transformation|GetActorLocation (.AsPlayer (Utilities|Casting|CastToBP_SHAKE_Player (PlayerState|GetPawn _array_element)))) "0.000000,0.000000,88.000000") _returnvalue) _explosionradius)
                  (Variables|/Game/Blueprints/Player/BP_SHAKE_Player.BP_SHAKE_Player_C|SetLastHitPlayer (.AsPlayer (Utilities|Casting|CastToBP_SHAKE_Player (PlayerState|GetPawn _array_element))) (select (== (.AsPlayer (Utilities|Casting|CastToBP_SHAKE_Player (PlayerState|GetPawn _array_element))) (Components|GetOwner)) (Variables|/Game/Blueprints/Player/BP_SHAKE_Player.BP_SHAKE_Player_C|GetLastHitPlayer (.AsPlayer (Utilities|Casting|CastToBP_SHAKE_Player (PlayerState|GetPawn _array_element)))) (.AsPlayer%20Controller (Utilities|Casting|CastToBP_SHAKE_PlayerController (Pawn|GetController (.AsPlayer (Utilities|Casting|CastToBP_SHAKE_Player (Components|GetOwner))))))))
                  (Default|Damage (.AsPlayer (Utilities|Casting|CastToBP_SHAKE_Player (PlayerState|GetPawn _array_element))) (* (/ (- _explosionradius (Math|Vector|Distance(Vector) (+ (Transformation|GetActorLocation (.AsPlayer (Utilities|Casting|CastToBP_SHAKE_Player (PlayerState|GetPawn _array_element)))) "0.000000,0.000000,88.000000") _returnvalue)) _explosionradius) (Variables|Projectile|GetSplashDamage)) (Math|Conversions|RotationFromXVector (Math|Vector|Normalize (- (Transformation|GetActorLocation (.AsPlayer (Utilities|Casting|CastToBP_SHAKE_Player (PlayerState|GetPawn _array_element)))) _returnvalue))) (== (.AsPlayer (Utilities|Casting|CastToBP_SHAKE_Player (PlayerState|GetPawn _array_element))) (Components|GetOwner))))))))
        (:then_1
          (CallFunction|MulticastSpawnExplosion)
          (Actor|DestroyActor))))))

(fn OnCollide
  (params (OtherActor :type Actor%20Object%20Reference) (Hit :type Hit%20Result%20Structure))
  (bind _returnvalue (Components|GetOwner))
  (bind (_bblockinghit _binitialoverlap _time _distance _location _impactpoint _normal _impactnormal) (Collision|BreakHitResult Hit))
  ;[0 0.3916 0.8963] Called when the projectile collides
  (Networking|SwitchHasAuthority
    (:Authority
      (bind _asplayer (Utilities|Casting|CastToBP_SHAKE_Player OtherActor)
        (:then
          (if (!= _asplayer _returnvalue)
            (Utilities|IsValid OtherActor
              (:Is%20Valid
                (Variables|/Game/Blueprints/Player/BP_SHAKE_Player.BP_SHAKE_Player_C|SetLastHitPlayer _asplayer (.AsPlayer%20Controller (Utilities|Casting|CastToBP_SHAKE_PlayerController (Pawn|GetController (.AsPlayer (Utilities|Casting|CastToBP_SHAKE_Player _returnvalue)))))))
              (:Is%20Not%20Valid
                _))
            (Default|Damage _asplayer (Variables|Projectile|GetContactDamage) (Math|Conversions|RotationFromXVector (Math|Vector|Normalize (- (+ "0.000000,0.000000,88.000000" (Transformation|GetActorLocation OtherActor)) (Transformation|GetActorLocation)))) false))
          (Projectile|Explode :!label _label))
        (:CastFailed
          (if (<= (Variables|Projectile|GetRemainingBounces) 0)
            (if (Class|GameplayStatics|ObjectIsA OtherActor "BP_SHAKE_Grenade_C")
              (goto _label)
              (else
                (CallFunction|MulticastSpawnBlastHole _impactpoint _impactnormal OtherActor)
                (goto _label)))
            (else
              (Math|Integer|DecrementInt (Variables|Projectile|GetRemainingBounces)
                (:%20%20
                  (CallFunction|MulticastPlayBumpSound (Transformation|GetActorLocation)))))))))))

(fn FollowPlayerVelocity
  (bind _returnvalue (Components|GetOwner))
  (bind _asplayer (Utilities|Casting|CastToBP_SHAKE_Player _returnvalue))
  (bind _charactermovement (Variables|/Script/Engine.Character|GetCharacterMovement _asplayer))
  ;[0 0.3813 0.8632] Follows the current velocity of the player
  (Utilities|IsValid (Components|GetOwner)
    (:Is%20Valid
      (if (> (Math|Vector|VectorLength (+ (Class|CharacterMovementComponent|GetImpartedMovementBaseVelocity _charactermovement) (Variables|/Script/Engine.MovementComponent|GetVelocity (Variables|Default|GetProjectileMovement)) (Variables|/Script/Engine.MovementComponent|GetVelocity _charactermovement))) (Math|Vector|VectorLength (Variables|/Script/Engine.MovementComponent|GetVelocity (Variables|Default|GetProjectileMovement))))
        (Variables|/Script/Engine.ProjectileMovementComponent|SetMaxSpeed (Variables|Default|GetProjectileMovement) (Math|Vector|VectorLength (+ (Class|CharacterMovementComponent|GetImpartedMovementBaseVelocity _charactermovement) (Variables|/Script/Engine.MovementComponent|GetVelocity (Variables|Default|GetProjectileMovement)) (Variables|/Script/Engine.MovementComponent|GetVelocity _charactermovement))))
        (Variables|/Script/Engine.MovementComponent|SetVelocity (Variables|Default|GetProjectileMovement) (* (Math|Vector|Normalize (Variables|/Script/Engine.MovementComponent|GetVelocity (Variables|Default|GetProjectileMovement))) (Math|Vector|VectorLength (+ (Class|CharacterMovementComponent|GetImpartedMovementBaseVelocity _charactermovement) (Variables|/Script/Engine.MovementComponent|GetVelocity (Variables|Default|GetProjectileMovement)) (Variables|/Script/Engine.MovementComponent|GetVelocity _charactermovement)))))))))