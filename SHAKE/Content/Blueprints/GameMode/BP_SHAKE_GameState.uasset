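; Game state for a SHAKE match, holding the replicated game rules, countdown timer and remaining-player count.
; The server loads host settings, and RepNotifies save rule changes, refresh client HUDs and check for a last-player win.
; When time expires, the server times players out, or on a kill tie starts sudden death by resetting lives so only tied leaders respawn.
; DoOnce gates keep each ending from repeating.
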(event Custom|CheckGameEnd
  ;[1 0.03955 0.03955] CHECK GAME END
  (Networking|SwitchHasAuthority
    (:Authority
      (if (and (== (Variables|Status|GetRemainingPlayers) 1) (Variables|Status|GetbHasStarted))
        (Utilities|FlowControl|DoOnce false
          (:Completed
            (Utilities|FlowControl|Delay 0.5)
            (for _array_element (Variables|Default|GetPlayerArray)
              (if (> (Variables|/Game/Blueprints/GameMode/BP_SHAKE_PlayerController.BP_SHAKE_PlayerController_C|GetLives (.AsPlayer%20Controller (Utilities|Casting|CastToBP_SHAKE_PlayerController (Game|GetPlayerController _array_element)))) 0)
                (Default|ClientWin (.AsPlayer%20Controller (Utilities|Casting|CastToBP_SHAKE_PlayerController (Game|GetPlayerController _array_element))))
                (else
                  (Default|ClientLose (.AsPlayer%20Controller (Utilities|Casting|CastToBP_SHAKE_PlayerController (Game|GetPlayerController _array_element))))))
              (CallFunction|MulticastSetTimer -1.0))))))))

(event Custom|Multicast_SetTimer
  (params (Timer :type Float%20%28double-precision%29))
  ;[1 0.03955 0.03955] TICK
  (Variables|Status|SetRemainingTime Timer))

(event Custom|Client_PlaySuddenDeathSound
  ;[1 0.03955 0.03955] PLAY SUDDEN DEATH SOUND
  (Audio|PlaySound2D "/Game/Sounds/VoiceLines/Announcer/SHAKE_Announcer_SuddenDeath.SHAKE_Announcer_SuddenDeath" (CallFunction|GetVoiceVolume) 1.0 0.0 0 0))

(event EventBeginPlay
  ;[0.956 0.0382 0.0382] BEGIN PLAY
  (|CallParentFunction)
  (Networking|SwitchHasAuthority
    (:Authority
      (Variables|GameRules|SetGameRules (.HostSettings (Utilities|Struct|BreakF_SHAKE_SaveData (Variables|/Game/Blueprints/GameManager/BP_SHAKE_GameManager.BP_SHAKE_GameManager_C|GetSaveData (CallFunction|GetGameManager))))))))

(event EventTick
  (params (DeltaSeconds :type Float%20%28single-precision%29))
  (bind (_btied _winningplayers) (SuddenDeath|IsTied))
  ;[1 0.03955 0.03955] TICK
  (|CallParentFunction DeltaSeconds)
  (if (> (Variables|Status|GetRemainingTime) 0.0)
    (bind _output_get (Variables|Status|SetRemainingTime (Math|Float|Max(Float) (- (Variables|Status|GetRemainingTime) DeltaSeconds) 0.0)))
    (Networking|SwitchHasAuthority
      (:Authority
        (if (== _output_get 0.0)
          (Utilities|FlowControl|DoOnce false
            (:Completed
              (CallFunction|MulticastSetTimer 0.0)
              (if _btied
                (SuddenDeath|SuddenDeath _winningplayers)
                (else
                  (for _array_element (Variables|Default|GetPlayerArray)
                    (Default|TimeOut (.AsPlayer%20Controller (Utilities|Casting|CastToBP_SHAKE_PlayerController (Game|GetPlayerController _array_element))))))))))))))

(fn ConstructionScript)

(fn OnRepGameRules
  (bind _player (CallFunction|MyPlayer))
  (bind _gamerules (Variables|GameRules|GetGameRules))
  (bind _availableweapons (Utilities|Struct|BreakF_SHAKE_GameRules _gamerules))
  (bind _hud (Variables|/Game/Blueprints/Player/BP_SHAKE_Player.BP_SHAKE_Player_C|GetHUD _player))
  ;[0 0.09759 0.5776] Replicates GameRules
  (Networking|SwitchHasAuthority
    (:Authority
      (bind _structout (Utilities|Struct|SetmembersinF_SHAKE_GameRules (Variables|GameRules|GetGameRules) (select (== _availableweapons 0) (Math|Conversions|ToByte(Integer) (|BitmaskLiteral 7)) _availableweapons)))
      (Utilities|Struct|SetmembersinF_SHAKE_SaveData (Variables|/Game/Blueprints/GameManager/BP_SHAKE_GameManager.BP_SHAKE_GameManager_C|GetSaveData (CallFunction|GetGameManager)) _structout))
    (:Remote
      (Utilities|IsValid _player
        (:Is%20Valid
          (Utilities|IsValid _hud
            (:Is%20Valid
              (Default|RefreshHUD _hud))))))))

(fn OnRepRemainingPlayers
  (bind _player (CallFunction|MyPlayer))
  (bind _hud (Variables|/Game/Blueprints/Player/BP_SHAKE_Player.BP_SHAKE_Player_C|GetHUD _player))
  ;[0.0137 0.7454 0.4179] Replicates the total number of remaining players
  (Utilities|FlowControl|Sequence
    (:then_0
      (Utilities|IsValid _player
        (:Is%20Valid
          (Utilities|IsValid _hud
            (:Is%20Valid
              (Default|UpdateRemainingPlayers _hud))))))
    (:then_1
      (Networking|SwitchHasAuthority
        (:Authority
          (CallFunction|CheckGameEnd))))))

(fn IsTied
  (bind __winningplayers (LocalVariables|Get_WinningPlayers))
  ;[0.2874 0 0] Returns whether a tie is currently in effect
  (Networking|SwitchHasAuthority
    (:Authority
      (for _array_element (Variables|Default|GetPlayerArray)
        (if (and (> (Variables|/Game/Blueprints/GameMode/BP_SHAKE_PlayerController.BP_SHAKE_PlayerController_C|GetCurrentKills (.AsPlayer%20Controller (Utilities|Casting|CastToBP_SHAKE_PlayerController (Game|GetPlayerController _array_element)))) (LocalVariables|Get_HighestKills)) (> (Variables|/Game/Blueprints/GameMode/BP_SHAKE_PlayerController.BP_SHAKE_PlayerController_C|GetLives (.AsPlayer%20Controller (Utilities|Casting|CastToBP_SHAKE_PlayerController (Game|GetPlayerController _array_element)))) 0))
          (LocalVariables|Set_HighestKills (Variables|/Game/Blueprints/GameMode/BP_SHAKE_PlayerController.BP_SHAKE_PlayerController_C|GetCurrentKills (.AsPlayer%20Controller (Utilities|Casting|CastToBP_SHAKE_PlayerController (Game|GetPlayerController _array_element)))))))
      (for _array_element_2 (Variables|Default|GetPlayerArray)
        (Utilities|Array|Add (select (and (== (Variables|/Game/Blueprints/GameMode/BP_SHAKE_PlayerController.BP_SHAKE_PlayerController_C|GetCurrentKills (.AsPlayer%20Controller (Utilities|Casting|CastToBP_SHAKE_PlayerController (Game|GetPlayerController (.AsPlayer%20State (Utilities|Casting|CastToBP_SHAKE_PlayerState _array_element_2)))))) (LocalVariables|Get_HighestKills)) (> (Variables|/Game/Blueprints/GameMode/BP_SHAKE_PlayerController.BP_SHAKE_PlayerController_C|GetLives (.AsPlayer%20Controller (Utilities|Casting|CastToBP_SHAKE_PlayerController (Game|GetPlayerController (.AsPlayer%20State (Utilities|Casting|CastToBP_SHAKE_PlayerState _array_element_2)))))) 0)) (LocalVariables|Get_WinningPlayers) (LocalVariables|Get_LosingPlayers)) (.AsPlayer%20State (Utilities|Casting|CastToBP_SHAKE_PlayerState _array_element_2))))
      (return (> (Utilities|Array|Length __winningplayers) 1) __winningplayers (LocalVariables|Get_LosingPlayers)))
    (:Remote
      (return false 0 0))))

(fn SuddenDeath
  (params (AlivePlayers :type Array%20of%20BP%20SHAKE%20Player%20State%20Object%20References))
  ;[0 0.402 0.9131] Begins sudden death
  (Networking|SwitchHasAuthority
    (:Authority
      (Utilities|FlowControl|DoOnce false
        (:Completed
          (for _array_element (Variables|Default|GetPlayerArray)
            (if (> (Variables|/Game/Blueprints/GameMode/BP_SHAKE_PlayerController.BP_SHAKE_PlayerController_C|GetLives (.AsPlayer%20Controller (Utilities|Casting|CastToBP_SHAKE_PlayerController (Game|GetPlayerController _array_element)))) 0)
              (Utilities|IsValid (Pawn|GetControlledPawn (.AsPlayer%20Controller (Utilities|Casting|CastToBP_SHAKE_PlayerController (Game|GetPlayerController _array_element))))
                (:Is%20Valid
                  (Variables|/Game/Blueprints/GameMode/BP_SHAKE_PlayerController.BP_SHAKE_PlayerController_C|SetLives (.AsPlayer%20Controller (Utilities|Casting|CastToBP_SHAKE_PlayerController (Game|GetPlayerController _array_element))) (Math|Integer|SelectInt 2 1 (Utilities|Array|ContainsItem AlivePlayers (.AsPlayer%20State (Utilities|Casting|CastToBP_SHAKE_PlayerState _array_element)))))
                  (Variables|/Game/Blueprints/Player/BP_SHAKE_Player.BP_SHAKE_Player_C|SetLastHitPlayer (.AsPlayer (Utilities|Casting|CastToBP_SHAKE_Player (Pawn|GetControlledPawn (.AsPlayer%20Controller (Utilities|Casting|CastToBP_SHAKE_PlayerController (Game|GetPlayerController _array_element)))))) 0)
                  (Default|Kill (.AsPlayer (Utilities|Casting|CastToBP_SHAKE_Player (Pawn|GetControlledPawn (.AsPlayer%20Controller (Utilities|Casting|CastToBP_SHAKE_PlayerController (Game|GetPlayerController _array_element)))))))
                  (Default|ClientForcePlayerStart (.AsPlayer%20Controller (Utilities|Casting|CastToBP_SHAKE_PlayerController (Game|GetPlayerController _array_element)))))
                (:Is%20Not%20Valid
                  (if (Utilities|Array|ContainsItem AlivePlayers (.AsPlayer%20State (Utilities|Casting|CastToBP_SHAKE_PlayerState _array_element)))
                    (Variables|/Game/Blueprints/GameMode/BP_SHAKE_PlayerController.BP_SHAKE_PlayerController_C|SetLives (.AsPlayer%20Controller (Utilities|Casting|CastToBP_SHAKE_PlayerController (Game|GetPlayerController _array_element))) 1)
                    (Default|ClientForcePlayerStart (.AsPlayer%20Controller (Utilities|Casting|CastToBP_SHAKE_PlayerController (Game|GetPlayerController _array_element))))
                    (else
                      (Variables|/Game/Blueprints/GameMode/BP_SHAKE_PlayerController.BP_SHAKE_PlayerController_C|SetLives (.AsPlayer%20Controller (Utilities|Casting|CastToBP_SHAKE_PlayerController (Game|GetPlayerController _array_element))) 0)
                      (Default|ClientCancelPlayerStart (.AsPlayer%20Controller (Utilities|Casting|CastToBP_SHAKE_PlayerController (Game|GetPlayerController _array_element))))))))))
          (CallFunction|ClientPlaySuddenDeathSound))))))