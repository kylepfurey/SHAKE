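; Game mode for SHAKE that picks player starts and lowers RemainingPlayers when a player with lives disconnects mid-match.
; Both start overrides cache eight slots ordered by PlayerStartTag and record the assigned controller.
; The main menu takes the first slot without an active pawn, linking any player display to its PlayerState.
; Matches favor the unclaimed start with the greatest summed squared distance to player pawns.
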(event Custom|PlayerDisconnected
  (params (Player :type Player%20Controller%20Object%20Reference))
  (bind _gamestate (CallFunction|GetGameState))
  ;[1 0.03955 0.03955] PLAYER DISCONNECTED
  (if (not (CallFunction|IsMainMenu))
    (if (> (Variables|/Game/Blueprints/GameMode/BP_SHAKE_PlayerController.BP_SHAKE_PlayerController_C|GetLives (.AsPlayer%20Controller (Utilities|Casting|CastToBP_SHAKE_PlayerController Player))) 0)
      (Variables|/Game/Blueprints/GameMode/BP_SHAKE_GameState.BP_SHAKE_GameState_C|SetRemainingPlayers _gamestate (Math|Integer|Max(Integer) (- (Variables|/Game/Blueprints/GameMode/BP_SHAKE_GameState.BP_SHAKE_GameState_C|GetRemainingPlayers _gamestate) 1) 1)))))

(fn ConstructionScript)

(fn ChoosePlayerStart
  (params (Player :type Controller%20Object%20Reference))
  (bind _playerstarts (Variables|Game|GetPlayerStarts))
  ;[0 0.4393 1] Returns the best player start
  (if (Utilities|Array|IsEmpty (Variables|Game|GetPlayerStarts))
    (for _index (range 0 7)
      (Utilities|Array|Add (Variables|Game|GetPlayerStarts) (Utilities|Struct|MakeF_SHAKE_PlayerStart 0 0)))
    (bind _outactors (Actor|GetAllActorsOfClass "/Script/Engine.PlayerStart"))
    (for _array_element _outactors
      (Utilities|Array|RemoveIndex _playerstarts (Math|Conversions|ToInteger(Byte) (Utilities|String|ToString(Name) (Variables|/Script/Engine.PlayerStart|GetPlayerStartTag _array_element))))
      (Utilities|Array|Insert _playerstarts (Utilities|Struct|MakeF_SHAKE_PlayerStart _array_element 0) (Math|Conversions|ToInteger(Byte) (Utilities|String|ToString(Name) (Variables|/Script/Engine.PlayerStart|GetPlayerStartTag _array_element))))))
  (if (CallFunction|IsMainMenu)
    (for (_array_element_2 _array_index) (Variables|Game|GetPlayerStarts)
      (Utilities|IsValid (.controller _array_element_2)
        (:Is%20Valid
          (Utilities|IsValid (Pawn|GetControlledPawn (.controller _array_element_2))
            (:Is%20Not%20Valid
              _)))
        (:Is%20Not%20Valid
          _))
      (bind _structout (Utilities|Struct|SetmembersinF_SHAKE_PlayerStart (Utilities|Array|Get(acopy) (Variables|Game|GetPlayerStarts) _array_index) Player))
      (Utilities|FlowControl|Sequence
        (:then_0
          (bind _asplayer_display (Utilities|Casting|CastToBP_SHAKE_PlayerDisplay (.playerstart _structout)))
          (Variables|/Game/Blueprints/Misc/BP_SHAKE_PlayerDisplay.BP_SHAKE_PlayerDisplay_C|SetPlayerState _asplayer_display (.AsPlayer%20State (Utilities|Casting|CastToBP_SHAKE_PlayerState (Variables|/Script/Engine.Controller|GetPlayerState (.controller _structout))))))
        (:then_1
          (return (.playerstart _structout)))))
    (bind _returnvalue (|CallParentFunction Player))
    (return _returnvalue)
    (else
      (bind _structout_2 (Utilities|Struct|SetmembersinF_SHAKE_PlayerStart (Utilities|Array|Get(acopy) (Variables|Game|GetPlayerStarts) (Game|GetRemotePlayerStartIndex)) Player))
      (return (.playerstart _structout_2)))))

(fn GetRemotePlayerStartIndex
  (bind _distances (LocalVariables|GetDistances))
  ;[0.0382 0.6376 0] Returns the index of the most remote player start
  (for _array_element (Variables|Game|GetPlayerStarts)
    (bind _returnvalue (Utilities|Array|Add _distances 0.0))
    (Utilities|IsValid (.controller _array_element)
      (:Is%20Not%20Valid
        (for _array_element_2 (Variables|/Script/Engine.GameStateBase|GetPlayerArray (CallFunction|GetGameState))
          (Utilities|IsValid _array_element_2
            (:Is%20Valid
              (Utilities|IsValid (PlayerState|GetPawn _array_element_2)
                (:Is%20Valid
                  (Utilities|Array|SetArrayElem (LocalVariables|GetDistances) _returnvalue (+ (Utilities|Array|Get(acopy) (LocalVariables|GetDistances) _returnvalue) (Class|KismetMathLibrary|VectorDistanceSquared (Transformation|GetActorLocation (PlayerState|GetPawn _array_element_2)) (Transformation|GetActorLocation (.playerstart _array_element)))))))))))))
  (for (_array_element_3 _array_index) _distances
    (if (> _array_element_3 (LocalVariables|GetGreatestDistance))
      (LocalVariables|SetGreatestDistance _array_element_3)
      (LocalVariables|SetGreatestDistanceIndex _array_index)))
  (return (LocalVariables|GetGreatestDistanceIndex)))

(fn FindPlayerStart
  (params (Player :type Controller%20Object%20Reference) (IncomingName :type String))
  (bind _playerstarts (Variables|Game|GetPlayerStarts))
  ;[0 0.4393 1] Returns the best player start
  (if (Utilities|Array|IsEmpty (Variables|Game|GetPlayerStarts))
    (for _index (range 0 7)
      (Utilities|Array|Add (Variables|Game|GetPlayerStarts) (Utilities|Struct|MakeF_SHAKE_PlayerStart 0 0)))
    (bind _outactors (Actor|GetAllActorsOfClass "/Script/Engine.PlayerStart"))
    (for _array_element _outactors
      (Utilities|Array|RemoveIndex _playerstarts (Math|Conversions|ToInteger(Byte) (Utilities|String|ToString(Name) (Variables|/Script/Engine.PlayerStart|GetPlayerStartTag _array_element))))
      (Utilities|Array|Insert _playerstarts (Utilities|Struct|MakeF_SHAKE_PlayerStart _array_element 0) (Math|Conversions|ToInteger(Byte) (Utilities|String|ToString(Name) (Variables|/Script/Engine.PlayerStart|GetPlayerStartTag _array_element))))))
  (if (CallFunction|IsMainMenu)
    (for (_array_element_2 _array_index) (Variables|Game|GetPlayerStarts)
      (Utilities|IsValid (.controller _array_element_2)
        (:Is%20Valid
          (Utilities|IsValid (Pawn|GetControlledPawn (.controller _array_element_2))
            (:Is%20Not%20Valid
              _)))
        (:Is%20Not%20Valid
          _))
      (bind _structout (Utilities|Struct|SetmembersinF_SHAKE_PlayerStart (Utilities|Array|Get(acopy) (Variables|Game|GetPlayerStarts) _array_index) Player))
      (Utilities|FlowControl|Sequence
        (:then_0
          (bind _asplayer_display (Utilities|Casting|CastToBP_SHAKE_PlayerDisplay (.playerstart _structout)))
          (Variables|/Game/Blueprints/Misc/BP_SHAKE_PlayerDisplay.BP_SHAKE_PlayerDisplay_C|SetPlayerState _asplayer_display (.AsPlayer%20State (Utilities|Casting|CastToBP_SHAKE_PlayerState (Variables|/Script/Engine.Controller|GetPlayerState (.controller _structout))))))
        (:then_1
          (return (.playerstart _structout)))))
    (bind _returnvalue (|CallParentFunction Player IncomingName))
    (return _returnvalue)
    (else
      (bind _structout_2 (Utilities|Struct|SetmembersinF_SHAKE_PlayerStart (Utilities|Array|Get(acopy) (Variables|Game|GetPlayerStarts) (Game|GetRemotePlayerStartIndex)) Player))
      (return (.playerstart _structout_2)))))