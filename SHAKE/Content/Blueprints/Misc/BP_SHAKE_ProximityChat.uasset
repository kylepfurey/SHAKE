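; BP_SHAKE_ProximityChat is a per-player voice talker component that provides attenuated proximity voice chat for BP_SHAKE_Player.
; It waits for a valid PlayerState, registers with it, and plays voices from the player's camera.
; The local player also registers as talker, gates the mic by settings and mute state, and activates audio capture in the main menu.
; Talk events apply the volume setting and toggle other players' chat icons.
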(event EventBPonTalkingEnd
  (bind _player (Variables|ProximityChat|GetPlayer))
  ;[1 0.03955 0.03955] END TALKING
  (|CallParentFunction)
  (Utilities|IsValid _player
    (:Is%20Valid
      (Rendering|SetVisibility (Variables|/Game/Blueprints/Player/BP_SHAKE_Player.BP_SHAKE_Player_C|GetChatIcon _player) false false))))

(event EventBPonTalkingBegin
  (params (AudioComponent :type Audio%20Component%20Object%20Reference))
  (bind _player (Variables|ProximityChat|GetPlayer))
  ;[1 0.03955 0.03955] BEGIN TALKING
  (Audio|Components|Audio|SetVolumeMultiplier AudioComponent (* (ProximityChat|GetProximityVolume) 2.0) :!class /Script/Engine.AudioComponent)
  (|CallParentFunction AudioComponent)
  (Utilities|IsValid _player
    (:Is%20Valid
      (if (and (Utilities|Enum|NotEqual(Enum) (Utilities|Struct|BreakF_SHAKE_PlayerSettings (CallFunction|GetPlayerSettings)) "NewEnumerator7") (!= _player (CallFunction|MyPlayer)))
        (Rendering|SetVisibility (Variables|/Game/Blueprints/Player/BP_SHAKE_Player.BP_SHAKE_Player_C|GetChatIcon _player) true false)))))

(event EventBeginPlay
  (bind _returnvalue (Components|GetOwner))
  (bind _asplayer (Utilities|Casting|CastToBP_SHAKE_Player _returnvalue))
  ;[1 0.03955 0.03955] BEGIN PLAY
  (|CallParentFunction)
  (bind _output_get (Variables|ProximityChat|SetPlayer _asplayer))
  (Utilities|IsValid (Variables|/Script/Engine.Pawn|GetPlayerState _output_get) :!label _label
    (:Is%20Valid
      (Class|VOIPTalker|RegisterwithPlayerState (Variables|/Script/Engine.Pawn|GetPlayerState _output_get))
      (Variables|Default|SetSettings (Utilities|Struct|MakeVoiceSettings (Variables|/Game/Blueprints/Player/BP_SHAKE_Player.BP_SHAKE_Player_C|GetCamera _output_get) "/Game/Sounds/Configuration/ProximityChatAttenuation.ProximityChatAttenuation" 0))
      (if (== _asplayer (CallFunction|MyPlayer))
        (Class|AdvancedVoiceLibrary|RegisterLocalTalker)
        (Class|VOIPStatics|SetMicThreshold (Math|Float|SelectFloat 0.05 1e+02 (and (Utilities|Enum|NotEqual(Enum) (Utilities|Struct|BreakF_SHAKE_PlayerSettings (CallFunction|GetPlayerSettings)) "NewEnumerator7") (not (Variables|/Game/Blueprints/GameManager/BP_SHAKE_GameManager.BP_SHAKE_GameManager_C|GetbMuted (CallFunction|GetGameManager))))))
        (if (CallFunction|IsMainMenu)
          (Components|Activation|Activate (Variables|/Game/Blueprints/Player/BP_SHAKE_Player.BP_SHAKE_Player_C|GetAudioCapture (Variables|ProximityChat|GetPlayer)) true))))
    (:Is%20Not%20Valid
      (Utilities|FlowControl|DelayUntilNextTick)
      (Utilities|IsValid self
        (:Is%20Valid
          (goto _label))))))

(fn GetProximityVolume
  ;[0.0382 0.6376 0] Returns the volume of proximity chat
  (return (Math|Conversions|ToFloat(Integer) (Utilities|String|EnumtoString (Utilities|Struct|BreakF_SHAKE_PlayerSettings (CallFunction|GetPlayerSettings))))))