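; BP_SHAKE_Gibs is the player's gib actor, showing body parts and gun in the player's colors, then destroying itself after a short delay.
; BeginPlay creates dynamic body, eye and gun materials, tints them with MetalColor and GlowColor, and applies them across the gib meshes.
; Outside LAN play, a SwitchOnLAN macro leads to fetching the Steam avatar for UniqueNetID and setting it as the eye texture.
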(event EventBeginPlay
  (bind _bodypivot (Variables|Default|GetBodyPivot))
  (bind _bodypivot_2 (Variables|Default|GetBodyPivot))
  (bind _gungib (Variables|Default|GetGunGib))
  (bind _glowcolor (Variables|Gibs|GetGlowColor))
  (bind _uniquenetid (Variables|Gibs|GetUniqueNetID))
  (bind _returnvalue (Math|Conversions|ToLinearColor(Color) _glowcolor))
  (bind _returnvalue_2 (Rendering|Material|GetMaterial _bodypivot 0))
  (bind _returnvalue_3 (Rendering|Material|GetMaterial _bodypivot_2 1))
  (bind _returnvalue_4 (Rendering|Material|GetMaterial _gungib 0))
  ;[0.9387 0.03689 0.03689] BEGIN PLAY
  (|CallParentFunction)
  (Utilities|FlowControl|Sequence
    (:then_0
      (bind _returnvalue_5 (Rendering|Material|CreateDynamicMaterialInstance _bodypivot 0 _returnvalue_2 (Utilities|String|StringToName (Utilities|GetDisplayName _returnvalue_2)) :!class /Script/Engine.PrimitiveComponent))
      (Variables|Gibs|SetBodyMaterial _returnvalue_5)
      (bind _returnvalue_6 (Rendering|Material|CreateDynamicMaterialInstance _bodypivot_2 1 _returnvalue_3 (Utilities|String|StringToName (Utilities|GetDisplayName _returnvalue_3)) :!class /Script/Engine.PrimitiveComponent))
      (Variables|Gibs|SetEyeMaterial _returnvalue_6)
      (bind _returnvalue_7 (Rendering|Material|CreateDynamicMaterialInstance _gungib 0 _returnvalue_4 (Utilities|String|StringToName (Utilities|GetDisplayName _returnvalue_4)) :!class /Script/Engine.PrimitiveComponent))
      (Variables|Gibs|SetGunMaterial _returnvalue_7)
      (Utilities|SwitchonLAN
        (:NotLAN
          (Class|AdvancedSteamFriendsLibrary|RequestSteamFriendInfo _uniquenetid false)
          (bind _returnvalue_8 (Class|AdvancedSteamFriendsLibrary|GetSteamFriendAvatar _uniquenetid (CallFunction|GetSteamAvatarSize))
            (:OnSuccess
              (Rendering|Material|SetTextureParameterValue (Variables|Gibs|GetEyeMaterial) "EyeTextureParam" _returnvalue_8))))))
    (:then_1
      (Rendering|Material|SetVectorParameterValue (Variables|Gibs|GetBodyMaterial) "MetalColorParam" (Math|Conversions|ToLinearColor(Color) (Variables|Gibs|GetMetalColor)) :!class /Script/Engine.MaterialInstanceDynamic)
      (Rendering|Material|SetVectorParameterValue (Variables|Gibs|GetBodyMaterial) "PlasticColorParam" _returnvalue :!class /Script/Engine.MaterialInstanceDynamic)
      (Rendering|Material|SetVectorParameterValue (Variables|Gibs|GetBodyMaterial) "PlasticColorParam" _returnvalue :!class /Script/Engine.MaterialInstanceDynamic)
      (Rendering|Material|SetMaterial (Variables|Default|GetLeftArmGib) 0 (Variables|Gibs|GetBodyMaterial))
      (Rendering|Material|SetMaterial (Variables|Default|GetHeadGib) 1 (Variables|Gibs|GetEyeMaterial))
      (Rendering|Material|SetMaterial (Variables|Default|GetGunGib) 0 (Variables|Gibs|GetGunMaterial)))
    (:then_2
      (Utilities|FlowControl|Delay 5.0)
      (Actor|DestroyActor))))

(fn ConstructionScript)