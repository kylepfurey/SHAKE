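; BP_SHAKE_KillFloor is a map actor that acts as an unbounded horizontal kill plane at its own Z height.
; Each tick, on authority only, it loops through the GameState PlayerArray and compares every valid pawn's Z with its own, without using overlaps.
; The KillAbove flag selects whether pawns at or above, or at or below, that height are cast to BP_SHAKE_Player and killed.
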(event EventTick
  (params (DeltaSeconds :type Float%20%28single-precision%29))
  (bind _returnvalue (Transformation|GetActorLocation))
  ;[1 0.03955 0.03955] TICK
  (|CallParentFunction DeltaSeconds)
  (Networking|SwitchHasAuthority
    (:Authority
      (for _array_element (Variables|/Script/Engine.GameStateBase|GetPlayerArray (CallFunction|GetGameState))
        (Utilities|IsValid (PlayerState|GetPawn _array_element)
          (:Is%20Valid
            (if (select (Variables|KillFloor|GetbKillAbove) (>= (.z (Transformation|GetActorLocation (PlayerState|GetPawn _array_element))) (.z _returnvalue)) (<= (.z (Transformation|GetActorLocation (PlayerState|GetPawn _array_element))) (.z _returnvalue)))
              (Default|Kill (.AsPlayer (Utilities|Casting|CastToBP_SHAKE_Player (PlayerState|GetPawn _array_element)))))))))))

(fn ConstructionScript)