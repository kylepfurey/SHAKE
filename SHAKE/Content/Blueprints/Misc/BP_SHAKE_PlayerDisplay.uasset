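; Main-menu display actor that shows a player's name, wins, losses and kills, hidden with collision off outside the menu.
; RefreshText reads the replicated PlayerState, or the local one when ClientOnly is set, blanking text if invalid or if PlayerState is the local player's.
; AppendLosses merges all three stats into the Wins line.
; Text refreshes on replication and in a randomly delayed polling loop.
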(event EventBeginPlay
  ;[0.9911 0.03955 0.03955] BEGIN PLAY
  (|CallParentFunction)
  (if (CallFunction|IsMainMenu)
    (PlayerDisplay|RefreshText :!label _label)
    (Utilities|FlowControl|Delay (Math|Random|RandomFloatinRange 0.1 1.0))
    (Utilities|IsValid self
      (:Is%20Valid
        (goto _label)))
    (else
      (Rendering|SetActorHiddenInGame true)
      (Collision|SetCollisionEnabled (Variables|Default|GetCube) "NoCollision"))))

(fn ConstructionScript)

(fn RefreshText
  (bind _playerstate (CallFunction|MyPlayerState))
  (bind _playerstate_2 (Variables|PlayerDisplay|GetPlayerState))
  (bind _bclientonly (Variables|PlayerDisplay|GetbClientOnly))
  (bind _returnvalue (select _bclientonly _playerstate _playerstate_2))
  (bind _kills (Variables|/Game/Blueprints/GameMode/BP_SHAKE_PlayerState.BP_SHAKE_PlayerState_C|GetKills _returnvalue))
  (bind _loses (Variables|/Game/Blueprints/GameMode/BP_SHAKE_PlayerState.BP_SHAKE_PlayerState_C|GetLoses _returnvalue))
  (bind _wins (Variables|/Game/Blueprints/GameMode/BP_SHAKE_PlayerState.BP_SHAKE_PlayerState_C|GetWins _returnvalue))
  (bind _returnvalue_2 (Utilities|String|ToString(Integer) _loses))
  (bind _returnvalue_3 (Utilities|String|ToString(Integer) _kills))
  (bind _returnvalue_4 (Utilities|String|ToString(Integer) _wins))
  (bind _returnvalue_5 (== _kills 1))
  (bind _returnvalue_6 (== _wins 1))
  (bind _returnvalue_7 (== _loses 1))
  (bind _returnvalue_8 (Utilities|String|SelectString " LOSS" " LOSSES" _returnvalue_7))
  (bind _returnvalue_9 (Utilities|String|SelectString " KILL" " KILLS" _returnvalue_5))
  (bind _returnvalue_10 (Utilities|String|SelectString " WIN" " WINS" _returnvalue_6))
  (bind _returnvalue_11 (Utilities|String|Append _returnvalue_3 _returnvalue_9))
  (bind _returnvalue_12 (Utilities|String|Append _returnvalue_4 _returnvalue_10))
  (bind _returnvalue_13 (Utilities|String|Append _returnvalue_2 _returnvalue_8))
  ;[0 0.3968 0.9047] Refreshes the player display based on the given player state
  (if (!= _playerstate_2 _playerstate)
    (Utilities|IsValid _returnvalue
      (:Is%20Valid
        (Rendering|Components|TextRender|SetText (Variables|Default|GetName) (Utilities|Text|ToText(String) (Utilities|String|ToString(Name) (Variables|/Game/Blueprints/GameMode/BP_SHAKE_PlayerState.BP_SHAKE_PlayerState_C|GetName _returnvalue))))
        (Rendering|Components|TextRender|SetText (Variables|Default|GetWins) (Utilities|Text|ToText(String) (Utilities|String|SelectString (Utilities|String|Append _returnvalue_12 " - " _returnvalue_13 " - " _returnvalue_11) _returnvalue_12 (Variables|PlayerDisplay|GetbAppendLosses))))
        (Rendering|Components|TextRender|SetText (Variables|Default|GetLoses) (Utilities|String|SelectText "" (Utilities|Text|ToText(String) _returnvalue_13) (Variables|PlayerDisplay|GetbAppendLosses)))
        (Rendering|Components|TextRender|SetText (Variables|Default|GetKills) (Utilities|String|SelectText "" (Utilities|Text|ToText(String) _returnvalue_11) (Variables|PlayerDisplay|GetbAppendLosses))))
      (:Is%20Not%20Valid
        (Rendering|Components|TextRender|SetText (Variables|Default|GetName) (Utilities|Text|MakeLiteralText "") :!label _label)))
    (else
      (goto _label))))

(fn OnRepPlayerState
  ;[0 0.402 0.9131] Replicates the player state
  (PlayerDisplay|RefreshText))